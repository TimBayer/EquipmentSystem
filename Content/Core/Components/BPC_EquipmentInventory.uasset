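; Equipment inventory component that turns item changes in its slots into equip and unequip events.
; On BeginPlay it binds to its inventory item added and removed events.
; Slot indices map to fixed equipment slots (chest, main hand, helmet, off hand, legs), broadcast through OnEquip and OnUnequip with the item.
; Added items must cast to CesEquipableItem, otherwise it only prints an error.
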(event EventBeginPlay
  (EventDispatchers|AssignOnInventoryItemAdded (EventDispatchers|CreateEvent :!event OnEquipmentAdded))
  (EventDispatchers|BindEventtoOnInventoryItemRemoved (EventDispatchers|CreateEvent :!event OnEquipmentRemoved)))

(fn OnEquipmentAdded
  (params (SlotIndex :type Integer) (Item :type Ces%20Item%20Data%20Structure))
  (bind _asces_equipable_item (Utilities|Casting|CastToCesEquipableItem (.Item (Utilities|Struct|BreakCesItemData Item)))
    (:then
      (Variables|Default|SetEquipableItem _asces_equipable_item)
      (switch int SlotIndex
        (:0
          (Default|CallOnEquip (Variables|Default|GetEquipableItem) "Chest"))
        (:1
          (Default|CallOnEquip (Variables|Default|GetEquipableItem) "MainHand"))
        (:2
          (Default|CallOnEquip (Variables|Default|GetEquipableItem) "Helmet"))
        (:3
          (Default|CallOnEquip (Variables|Default|GetEquipableItem) "OffHand"))
        (:4
          (Default|CallOnEquip (Variables|Default|GetEquipableItem) "Legs"))))
    (:CastFailed
      (Development|PrintString "BPC_EquipmentInventory: Item not Equipable Item!" true true "(R=1.000000,G=0.000000,B=0.000000,A=1.000000)"))))

(fn OnEquipmentRemoved
  (params (SlotIndex :type Integer) (Item :type Ces%20Item%20Data%20Structure))
  (LocalVariables|SetRemovedItem Item)
  (switch int SlotIndex
    (:0
      (Default|CallOnUnequip "Chest" (LocalVariables|GetRemovedItem)))
    (:1
      (Default|CallOnUnequip "MainHand" (LocalVariables|GetRemovedItem)))
    (:2
      (Default|CallOnUnequip "Helmet" (LocalVariables|GetRemovedItem)))
    (:3
      (Default|CallOnUnequip "OffHand" (LocalVariables|GetRemovedItem)))
    (:4
      (Default|CallOnUnequip "Legs" (LocalVariables|GetRemovedItem)))))