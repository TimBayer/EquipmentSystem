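; BPC_Stats is a component that keeps running Damage and Armor totals, apparently from equipment.
; AddStats and RemoveStats add or subtract the values of a passed stats struct to or from those totals.
; After each change it broadcasts StatsUpdated with the new totals packed into a CesEquipmentStats struct, so listeners receive the current values.
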(fn AddStats
  (params (Stats :type Ces%20Equipment%20Stats%20Structure))
  (bind (_damage _armor) (Utilities|Struct|BreakCesEquipmentStats Stats))
  (Variables|Default|SetDamage (+ (Variables|Default|GetDamage) _damage))
  (Variables|Default|SetArmor (+ (Variables|Default|GetArmor) _armor))
  (Default|CallStatsUpdated (Utilities|Struct|MakeCesEquipmentStats (Variables|Default|GetDamage) (Variables|Default|GetArmor))))

(fn RemoveStats
  (params (Stats :type Ces%20Equipment%20Stats%20Structure))
  (bind (_damage _armor) (Utilities|Struct|BreakCesEquipmentStats Stats))
  (Variables|Default|SetDamage (- (Variables|Default|GetDamage) _damage))
  (Variables|Default|SetArmor (- (Variables|Default|GetArmor) _armor))
  (Default|CallStatsUpdated (Utilities|Struct|MakeCesEquipmentStats (Variables|Default|GetDamage) (Variables|Default|GetArmor))))