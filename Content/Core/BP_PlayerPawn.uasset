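; Player pawn with a Spine-animated skeleton and equipment that changes stats and appearance.
; A/D play run or idle and flip facing, while Space layers a looping shoot animation on a second track; no movement or firing logic exists here.
; Equipment inventory events are bound on BeginPlay.
; Equip and unequip handlers update BPCStats and spawn or destroy per-slot equipment actors, each given a Spine bone name to target.
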(event EventBeginPlay
  (Input|EnableInput (Game|GetPlayerController 0))
  (Class|SpineSkeletonAnimationComponent|SetAnimation (Variables|Default|GetSkeletonAnimationComponent) 0 "idle" true)
  ;[1 1 1] Bind to Equipment change events
  (EventDispatchers|BindEventtoOnEquip (Variables|Default|GetEquipmentInventory) (EventDispatchers|CreateEvent :!event OnEquipItem))
  (EventDispatchers|BindEventtoOnUnequip (Variables|Default|GetEquipmentInventory) (EventDispatchers|CreateEvent :!event OnUnequipItem)))

(event Input|KeyboardEvents|D
  (params (Key :type Key%20Structure :default "None"))
  ;[1 1 1] Run Right
  (:Pressed
    (Class|SpineSkeletonComponent|SetScaleX (Variables|Default|GetSkeletonAnimationComponent) 1.0)
    (Class|SpineSkeletonAnimationComponent|SetAnimation (Variables|Default|GetSkeletonAnimationComponent) 0 "run" true))
  (:Released
    (Class|SpineSkeletonAnimationComponent|SetAnimation (Variables|Default|GetSkeletonAnimationComponent) 0 "idle" true)))

(event Input|KeyboardEvents|A
  (params (Key :type Key%20Structure :default "None"))
  ;[1 1 1] Run Left
  (:Pressed
    (Class|SpineSkeletonComponent|SetScaleX (Variables|Default|GetSkeletonAnimationComponent) -1.0)
    (Class|SpineSkeletonAnimationComponent|SetAnimation (Variables|Default|GetSkeletonAnimationComponent) 0 "run" true))
  (:Released
    (Class|SpineSkeletonAnimationComponent|SetAnimation (Variables|Default|GetSkeletonAnimationComponent) 0 "idle" true)))

(event Input|KeyboardEvents|SpaceBar
  (params (Key :type Key%20Structure :default "None"))
  ;[1 1 1] Shoot
  (:Pressed
    (Class|SpineSkeletonAnimationComponent|SetAnimation (Variables|Default|GetSkeletonAnimationComponent) 1 "shoot" true))
  (:Released
    (Class|SpineSkeletonAnimationComponent|SetEmptyAnimation (Variables|Default|GetSkeletonAnimationComponent) 1 0.2)))

(fn ConstructionScript)

(fn OnEquipItem
  (params (EquipmentItem :type Ces%20Equipable%20Item%20Object%20Reference) (EquipmentSlot :type EEquipmentSlotType%20Enum :default "MainHand"))
  ;[1 1 1] Update Stats
  (Default|AddStats (Variables|Default|GetBPC_Stats) (Variables|/Script/EquipmentSystem.CesEquipableItem|GetStats EquipmentItem))
  (bind _asbp_equipment_base (Utilities|Casting|CastToBP_Equipment_BaseClass (Variables|/Script/EquipmentSystem.CesEquipableItem|GetEquipmentActor EquipmentItem)))
  (LocalVariables|SetEquipmentActor _asbp_equipment_base)
  ;[1 1 1] Spawn Equipment Actor
  (switch Utilities|FlowControl|Switch|SwitchonEEquipmentSlotType EquipmentSlot
    (:MainHand
      (CallFunction|SpawnEquipment "MainHand" (LocalVariables|GetEquipmentActor) "gun"))
    (:OffHand
      (CallFunction|SpawnEquipment "OffHand" (LocalVariables|GetEquipmentActor) "front-fist"))
    (:Helmet
      (CallFunction|SpawnEquipment "Helmet" (LocalVariables|GetEquipmentActor) "head"))
    (:Chest
      (CallFunction|SpawnEquipment "Chest" (LocalVariables|GetEquipmentActor) "torso"))
    (:Legs
      (CallFunction|SpawnEquipment "Legs" (LocalVariables|GetEquipmentActor) "front-thigh"))))

(fn SpawnEquipment
  (params (EquipmentSlot :type EEquipmentSlotType%20Enum :default "MainHand") (EquipmentActorClass :type BP%20Equipment%20Base%20Class%20Reference) (SpineBoneName :type String))
  (bind _self self)
  (bind _returnvalue (Game|SpawnActorfromClass EquipmentActorClass (Math|Transform|MakeTransform "0, 0, 0") "Undefined" _self _self SpineBoneName 0))
  (LocalVariables|SetEquipmentActor _returnvalue)
  (switch Utilities|FlowControl|Switch|SwitchonEEquipmentSlotType EquipmentSlot
    (:MainHand
      (Variables|Equipment|SetMainHand (LocalVariables|GetEquipmentActor)))
    (:OffHand
      (Variables|Equipment|SetOffHand (LocalVariables|GetEquipmentActor)))
    (:Helmet
      (Variables|Equipment|SetHelmet (LocalVariables|GetEquipmentActor)))
    (:Chest
      (Variables|Equipment|SetChest (LocalVariables|GetEquipmentActor)))
    (:Legs
      (Variables|Equipment|SetLegs (LocalVariables|GetEquipmentActor)))))

(fn OnUnequipItem
  (params (EquipmentSlot :type EEquipmentSlotType%20Enum :default "MainHand") (UnequippedItem :type Ces%20Item%20Data%20Structure))
  ;[1 1 1] Update Stats
  (bind _asces_equipable_item (Utilities|Casting|CastToCesEquipableItem (.Item (Utilities|Struct|BreakCesItemData UnequippedItem))))
  (Default|RemoveStats (Variables|Default|GetBPC_Stats) (Variables|/Script/EquipmentSystem.CesEquipableItem|GetStats _asces_equipable_item))
  ;[1 1 1] Remove Equipment Actor
  (switch Utilities|FlowControl|Switch|SwitchonEEquipmentSlotType EquipmentSlot
    (:MainHand
      (Actor|DestroyActor (Variables|Equipment|GetMainHand)))
    (:OffHand
      (Actor|DestroyActor (Variables|Equipment|GetOffHand)))
    (:Helmet
      (Actor|DestroyActor (Variables|Equipment|GetHelmet)))
    (:Chest
      (Actor|DestroyActor (Variables|Equipment|GetChest)))
    (:Legs
      (Actor|DestroyActor (Variables|Equipment|GetLegs)))))