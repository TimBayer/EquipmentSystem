(event EventBeginPlay
  (Utilities|FlowControl|Delay 0.2)
  (bind _asbp_hud (Utilities|Casting|CastToBP_HUD (HUD|GetHUD)))
  (Variables|Default|SetPlayerHUD _asbp_hud)
  (|LoadStartingItems))

(event Input|KeyboardEvents|F
  (params (Key :type Key%20Structure :default "None"))
  (:Pressed
    (|FillMoreAssets)))

(event Input|KeyboardEvents|I
  (params (Key :type Key%20Structure :default "None"))
  (:Pressed
    (Default|ToggleInventoryDisplay (Variables|Default|GetPlayerHUD))))

(fn ConstructionScript)